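; Player-controlled flying airship Character that sets flying movement on begin play and moves along its forward, right and up axes from input.
; Mouse axes orbit the spring arm camera independently of the hull.
; The roll axis feeds a turn speed with exponential, delta-time-based damping that drives controller yaw.
; Holding secondary attack also steers the ship toward the camera's heading, passing the wrapped yaw difference through a curve.
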(event `self.ReceiveBeginPlay`
  (`CharacterMovementComponent.SetMovementMode` (`self.CharacterMovement`) "MOVE_Flying" 0))

(event `self.ReceiveTick`
  (params (DeltaSeconds :type "Float (single-precision)"))
  (bind (_returnvalue_roll _returnvalue_pitch _returnvalue_yaw) (`KismetMathLibrary.BreakRotator` (`SceneComponent.K2_GetComponentRotation` (`self.CapsuleComponent`))))
  (bind (_returnvalue_roll_2 _returnvalue_pitch_2 _returnvalue_yaw_2) (`KismetMathLibrary.BreakRotator` (`SceneComponent.K2_GetComponentRotation` (`self.SpringArm`))))
  (bind _returnvalue (mod (+ (- _returnvalue_yaw_2 _returnvalue_yaw) 360.0) 360.0))
  (if (`self.mouse turning`)
    (bind _output_get (set `self.turn speed` (* (+ (* (`CurveFloat.GetFloatValue` (`self.turn speed curve`) (select `bool` (>= _returnvalue 180.0) :`false` _returnvalue :`true` (- _returnvalue 360.0))) DeltaSeconds 0.2) (`self.turn speed`)) (`KismetMathLibrary.MultiplyMultiply_FloatFloat` 0.3 DeltaSeconds))))
    (`self.AddControllerYawInput` _output_get)))

(event `InputAction|secondary attack`
  (params (Key :type "Key Structure"))
  (:`Pressed`
    (set `self.mouse turning` true))
  (:`Released`
    (set `self.mouse turning` false)))

(event `InputAxis|vertical`
  (params (AxisValue :type "Float (single-precision)"))
  (`self.AddMovementInput` (`self.GetActorUpVector`) AxisValue))

(event `InputAxis|roll`
  (params (AxisValue :type "Float (single-precision)"))
  (bind _returnvalue (`GameplayStatics.GetWorldDeltaSeconds`))
  (bind _output_get (set `self.turn speed` (* (+ (* AxisValue _returnvalue 0.2) (`self.turn speed`)) (`KismetMathLibrary.MultiplyMultiply_FloatFloat` 0.3 _returnvalue))))
  (`self.AddControllerYawInput` _output_get))

(event `InputAxis|forward`
  (params (AxisValue :type "Float (single-precision)"))
  (`self.AddMovementInput` (`self.GetActorForwardVector`) AxisValue))

(event `InputAxis|sideways`
  (params (AxisValue :type "Float (single-precision)"))
  (`self.AddMovementInput` (`self.GetActorRightVector`) AxisValue))

(event `InputAxis|mouse y`
  (params (AxisValue :type "Float (single-precision)"))
  (bind _springarm (`self.SpringArm`))
  (`SceneComponent.K2_AddWorldRotation` _springarm (`KismetMathLibrary.RotatorFromAxisAndAngle` (`SceneComponent.GetRightVector` _springarm) AxisValue) false false))

(event `InputAxis|mouse x`
  (params (AxisValue :type "Float (single-precision)"))
  (`SceneComponent.K2_AddWorldRotation` (`self.SpringArm`) (`KismetMathLibrary.RotatorFromAxisAndAngle` (`self.GetActorUpVector`) AxisValue) false false))

(fn `UserConstructionScript`)